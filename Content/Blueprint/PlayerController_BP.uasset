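; Player controller for the wizard character, combining click-to-move, axis movement and orbit camera control.
; Middle-click spawns a goal decal under the cursor and starts SimpleMoveToLocation, replacing any previous command.
; While EnableTurning is held, look axes rotate the camera arm with clamped pitch.
; Movement axes act only during a click command, cancelling it and adding camera-yaw-relative input, with MoveRight ignoring axis sign.
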(event `self.ReceiveBeginPlay`
  (bind _aswizard_character (cast `/Game/Blueprint/Character/Wizard/Wizard_Character` (`self.K2_GetPawn`)))
  (set `self.Controlled Char` _aswizard_character))

(event `InputAction|EnableTurning`
  (params (Key :type "Key Structure"))
  (:`Pressed`
    (set `self.ChaTurn?` true))
  (:`Released`
    (set `self.ChaTurn?` false)))

(event `InputAxis|LookUp`
  (params (AxisValue :type "Float (single-precision)"))
  (bind _cameraarm (`/Game/Blueprint/Character/Wizard/Wizard_Character.CameraArm` (`self.Controlled Char`)))
  (if (and (!= AxisValue 0.0) (`self.ChaTurn?`))
    (`SceneComponent.K2_SetRelativeRotation` _cameraarm (`KismetMathLibrary.MakeRotator` (.roll (.rotation (`SceneComponent.GetRelativeTransform` _cameraarm))) (`KismetMathLibrary.FClamp` (+ (.pitch (.rotation (`SceneComponent.GetRelativeTransform` _cameraarm))) (* AxisValue 1.5)) -40.0 0.0) (.yaw (.rotation (`SceneComponent.GetRelativeTransform` _cameraarm)))) false false)))

(event `InputAxis|Turn`
  (params (AxisValue :type "Float (single-precision)"))
  (bind _cameraarm (`/Game/Blueprint/Character/Wizard/Wizard_Character.CameraArm` (`self.Controlled Char`)))
  (if (and (!= AxisValue 0.0) (`self.ChaTurn?`))
    (`SceneComponent.K2_SetRelativeRotation` _cameraarm (`KismetMathLibrary.MakeRotator` (.roll (.rotation (`SceneComponent.GetRelativeTransform` _cameraarm))) (.pitch (.rotation (`SceneComponent.GetRelativeTransform` _cameraarm))) (+ (.yaw (.rotation (`SceneComponent.GetRelativeTransform` _cameraarm))) (* AxisValue 2.0))) false false)))

(event `Key|MiddleMouseButton`
  (params (Key :type "Key Structure"))
  (bind (_bblockinghit _binitialoverlap _time _distance _location) (`GameplayStatics.BreakHitResult` (`self.GetHitResultUnderCursorByChannel` "TraceTypeQuery1")))
  (:`Pressed`
    (`self.CancelMovementCommand`)
    (bind _returnvalue (`|SpawnActorFromClass` "/Game/SkillSystem/Blueprint/GoalDecal_BP.GoalDecal_BP_C" (`KismetMathLibrary.Conv_VectorToTransform` _location) "Undefined" "OverrideRootScale" null self null))
    (set `self.CurrentGoaldecal` _returnvalue)
    (set `self.HasMouseMovementCommand?` true)
    (`AIBlueprintHelperLibrary.SimpleMoveToLocation` self _location)))

(event `InputAxis|MoveForward`
  (params (AxisValue :type "Float (single-precision)"))
  (bind _controlled_char (`self.Controlled Char`))
  (if (!= AxisValue 0.0)
    (if (`self.HasMouseMovementCommand?`)
      (`self.CancelMovementCommand`)
      (`Pawn.AddMovementInput` _controlled_char (`KismetMathLibrary.GetForwardVector` (`KismetMathLibrary.MakeRotator` 0.0 0.0 (.yaw (.rotation (`SceneComponent.GetRelativeTransform` (`/Game/Blueprint/Character/Wizard/Wizard_Character.CameraArm` _controlled_char)))))) AxisValue false))))

(event `InputAxis|MoveRight`
  (params (AxisValue :type "Float (single-precision)"))
  (bind _controlled_char (`self.Controlled Char`))
  (if (!= AxisValue 0.0)
    (if (`self.HasMouseMovementCommand?`)
      (`self.CancelMovementCommand`)
      (`Pawn.AddMovementInput` _controlled_char (`KismetMathLibrary.GetRightVector` (`KismetMathLibrary.MakeRotator` 0.0 0.0 (.yaw (.rotation (`SceneComponent.GetRelativeTransform` (`/Game/Blueprint/Character/Wizard/Wizard_Character.CameraArm` _controlled_char)))))) 1.0 false))))

(fn `CancelMovementCommand`
  (`/Engine/EditorBlueprintResources/StandardMacros.IsValid` (`self.CurrentGoaldecal`)
    (:`Is Valid`
      (`MovementComponent.StopMovementImmediately` (`Character.CharacterMovement` (`self.Controlled Char`)))
      (`self.K2_DestroyActor` (`self.CurrentGoaldecal`))
      (set `self.HasMouseMovementCommand?` false)
      (set `self.CurrentGoaldecal` null))
    (:`Is Not Valid`
      _))
  (return))

(fn `UserConstructionScript`)