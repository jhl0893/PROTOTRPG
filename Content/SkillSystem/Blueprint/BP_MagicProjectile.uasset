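; BP_MagicProjectile is a homing skill missile that flies at a target and deals the spell's damage on hit.
; On BeginPlay it takes its speed from the Skill's current stage, applies the missile particle effect and homes on the target's HItArrow component.
; When its sphere overlaps that target's capsule, it spawns an impact emitter, passes stage damage, type, crit chance and skill element to OnReceiveDamage, then destroys itself.
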(event `self.ReceiveBeginPlay`
  (bind _projectilemovement (`self.ProjectileMovement`))
  (bind ((`MissileSpeed_39_A8DCC3F14BCD4932C2AD578DDD7DE477` _missilespeed)) (break `/Game/SkillSystem/Enum_Structure/s_SkillStage` (`/Game/SkillSystem/Blueprint/Master_Skill.GetCurrentStage` (`self.Skill`))))
  (set `ProjectileMovementComponent.InitialSpeed` _missilespeed _projectilemovement)
  (set `ProjectileMovementComponent.MaxSpeed` _missilespeed _projectilemovement)
  (`ParticleSystemComponent.SetTemplate` (`self.ParticleSystem`) (`self.MissileEffect`))
  (set `ProjectileMovementComponent.HomingTargetComponent` (`/Game/Blueprint/Character/Monster/Mon_Character.HIt Arrow` (`self.Target`)) (`self.ProjectileMovement`)))

(event `self.Sphere.OnComponentBeginOverlap`
  (params (OverlappedComponent :type "PrimitiveComponent Object Reference") (OtherActor :type "Actor Object Reference") (OtherComp :type "PrimitiveComponent Object Reference") (OtherBodyIndex :type Integer) (bFromSweep :type Boolean) (SweepResult :type "HitResult Structure (by ref)"))
  (bind _skill (`self.Skill`))
  (bind _skill_2 (`self.Skill`))
  (bind ((`Damage_22_ABE5951C4DD5E9E4C7FAD0877D4A5191` _damage) (`DamageType_25_90B3CB904FD02089E3AEA795488D61A1` _damagetype) (`CriticalChanace_28_D614AF67444C66FB89E34AA098063A04` _criticalchanace)) (break `/Game/SkillSystem/Enum_Structure/s_SkillStage` (`/Game/SkillSystem/Blueprint/Master_Skill.GetCurrentStage` _skill)))
  (if (and (== OtherActor (`self.Target`)) (== (`GameplayStatics.GetObjectClass` OtherComp) "/Script/Engine.CapsuleComponent"))
    (`GameplayStatics.SpawnEmitterAtLocation` (`self.ImpactEffect`) (`self.K2_GetActorLocation`) (struct) (1.0 1.0 1.0) true "None" false)
    (`/Game/Blueprint/Character/Monster/Mon_Character.OnReceiveDamage` (`self.Target`) _damage _damagetype (`.Element_16_6F953E954226D9EB1EB6B4BA19F14042` (break `/Game/SkillSystem/Enum_Structure/s_SkillInfo` (`/Game/SkillSystem/Blueprint/Master_Skill.SKillInfo` _skill))) _criticalchanace (`/Game/SkillSystem/Blueprint/Master_Skill.PlayerREF` _skill_2) _skill_2)
    (`self.K2_DestroyActor`)))

(fn `UserConstructionScript`)