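; Area-of-effect skill that damages pawns around the player.
; On the skill notify it spawns a particle effect at the player's location and runs a zero-length multi sphere trace there, sized by the current stage's radius and ignoring the player.
; Each hit implementing the Damage interface receives a damage message with the stage's damage, type and crit chance, plus the skill's element.
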(event `self.OnSkillNotify`
  (bind _playerref (`self.PlayerREF`))
  (bind ((`Damage_22_ABE5951C4DD5E9E4C7FAD0877D4A5191` _damage) (`DamageType_25_90B3CB904FD02089E3AEA795488D61A1` _damagetype) (`CriticalChanace_28_D614AF67444C66FB89E34AA098063A04` _criticalchanace)) (break `/Game/SkillSystem/Enum_Structure/s_SkillStage` (`self.GetCurrentStage`)))
  (bind _returnvalue (`self.K2_GetActorLocation` _playerref))
  (`GameplayStatics.SpawnEmitterAtLocation` (`self.ParticleEffect`) _returnvalue)
  (bind _outhits (`KismetSystemLibrary.SphereTraceMultiForObjects` _returnvalue _returnvalue (`.AreaRadius_37_A03F731241B3940105071DB73B6B0341` (break `/Game/SkillSystem/Enum_Structure/s_SkillStage` (`self.GetCurrentStage`))) (`|MakeArray` "ObjectTypeQuery3" :!type "EObjectTypeQuery Enum") true (`|MakeArray` _playerref :!type "Actor Object Reference")))
  (for _array_element _outhits
    (bind (_bblockinghit _binitialoverlap _time _distance _location _impactpoint _normal _impactnormal _physmat _hitactor) (`GameplayStatics.BreakHitResult` _array_element))
    (if (`KismetSystemLibrary.DoesImplementInterface` _hitactor "/Game/SkillSystem/Blueprint/Damage.Damage_C")
      (message `/Game/SkillSystem/Blueprint/Damage.OnReceiveDamage` _hitactor _damage _damagetype (`.Element_16_6F953E954226D9EB1EB6B4BA19F14042` (break `/Game/SkillSystem/Enum_Structure/s_SkillInfo` (`self.SKillInfo`))) _criticalchanace (`self.PlayerREF`) self))))

(fn `UserConstructionScript`
  (`parent.UserConstructionScript`))