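; Targeted missile skill that fires a BP_MagicProjectile at the player's selected enemy.
; When out of range, a looping timer moves the player toward the enemy and registers the skill on the controller until in range or the target is invalid.
; Casting checks and spends stage-based mana, turns the player toward the enemy and calls the parent cast logic.
; The skill notify spawns the projectile with its effects if the target is alive.
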(event `StopTimer`
  (`KismetSystemLibrary.K2_ClearAndInvalidateTimerHandle` (`self.DistanceTimer`))
  (set `/Game/Blueprint/PlayerController_BP.MissileSpell` null (`/Game/Blueprint/Character/Wizard/Wizard_Character.PlayerControlREF` (`self.PlayerREF`))))

(event `self.OnTryCastSpell`
  (bind _playerref (`self.PlayerREF`))
  (bind _selectedenemy (`/Game/Blueprint/Character/Wizard/Wizard_Character.SelectedEnemy` _playerref))
  (if (and (not (`self.OnCoolDown?`)) (not (`self.Currently Casted?`)) (not (`/Game/Blueprint/Character/Wizard/Wizard_Character.isCasting?` _playerref)) (`KismetSystemLibrary.IsValid` _selectedenemy))
    (set `self.Selected Enemy` _selectedenemy)
    (`self.Initialize SpellCast`)))

(event `self.Initialize SpellCast`
  (if (`self.InAttackRange`)
    (`self.ManaCheck`)
    (else
      (bind _returnvalue (`KismetSystemLibrary.K2_SetTimer` self "DistanceCheck" 0.2 true))
      (set `self.DistanceTimer` _returnvalue)
      (set `/Game/Blueprint/PlayerController_BP.MissileSpell` self (`/Game/Blueprint/Character/Wizard/Wizard_Character.PlayerControlREF` (`self.PlayerREF`))))))

(event `ManaCheck`
  (bind _playerref (`self.PlayerREF`))
  (bind ((`ManaCost_44_4C078B0A4A4028F864CEA09F3DA6E744` _manacost)) (break `/Game/SkillSystem/Enum_Structure/s_SkillStage` (`self.GetCurrentStage`)))
  (if (>= (`.CurrentValue_7_2F63A7F6498A3A7B352ACBAAB7C9183F` (break `/Game/SkillSystem/Enum_Structure/s_StatData` (`/Game/Blueprint/Character/Wizard/Wizard_Character.GetStat` (`self.PlayerREF`) "NewEnumerator2"))) _manacost)
    (set `self.Currently Casted?` true)
    (`/Game/Blueprint/Character/Wizard/Wizard_Character.BeginSpellCast` _playerref self)
    (`/Game/Blueprint/Character/Wizard/Wizard_Character.ModifyStat` _playerref "NewEnumerator2" (* _manacost -1) true)
    (`self.OnSpellCast`)
    (else
      (`KismetSystemLibrary.PrintString` "nor enought mana" true true (struct :`R` 1.0 :`B` 0.092422 :`A` 1.0)))))

(event `self.OnSpellCast`
  (bind _playerref (`self.PlayerREF`))
  (`self.K2_SetActorRotation` _playerref (`KismetMathLibrary.FindLookAtRotation` (`self.K2_GetActorLocation` _playerref) (`self.K2_GetActorLocation` (`self.Selected Enemy`))) false)
  (`parent.OnSpellCast`))

(event `self.OnSkillNotify`
  (if (not (`/Game/Blueprint/Character/Monster/Mon_Character.IsDead?` (`self.Selected Enemy`)))
    (`|SpawnActorFromClass` "/Game/SkillSystem/Blueprint/BP_MagicProjectile.BP_MagicProjectile_C" (`KismetMathLibrary.MakeTransform` (+ (`self.K2_GetActorLocation` (`self.PlayerREF`)) (0.0 0.0 80.0))) "Undefined" "OverrideRootScale" null (`self.Selected Enemy`) self (`self.MissileEffect`) (`self.impactEffect`) null)))

(fn `DistanceCheck`
  (bind _selectedenemy (`/Game/Blueprint/Character/Wizard/Wizard_Character.SelectedEnemy` (`self.PlayerREF`)))
  (`/Engine/EditorBlueprintResources/StandardMacros.IsValid` _selectedenemy
    (:`Is Valid`
      (if (`self.InAttackRange`)
        (`self.StopTimer`)
        (`self.ManaCheck`)
        (else
          (`AIBlueprintHelperLibrary.SimpleMoveToActor` (`/Game/Blueprint/Character/Wizard/Wizard_Character.PlayerControlREF` (`self.PlayerREF`)) _selectedenemy))))
    (:`Is Not Valid`
      (`self.StopTimer`))))

(fn `InAttackRange`
  (returns (`out?` :type Boolean))
  (bind _playerref (`self.PlayerREF`))
  (return (<= (`self.GetDistanceTo` _playerref (`/Game/Blueprint/Character/Wizard/Wizard_Character.SelectedEnemy` _playerref)) (`.Range_20_1BDA91624104F67B4FA41E8F1EAC36D8` (break `/Game/SkillSystem/Enum_Structure/s_SkillStage` (`self.GetCurrentStage`))))))

(fn `UserConstructionScript`
  (`parent.UserConstructionScript`))