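; Base skill Blueprint that runs a player spell's cast and cooldown cycle.
; A cast requires no cooldown or active cast and enough mana, which it deducts before starting.
; The montage is rate-scaled to the current stage's cast time, locking movement while a timeline fills the casting bar.
; On completion, a second timeline runs the cooldown, updating the hotkey's radial material and countdown text until the skill re-enables.
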(event `OnSpellCast`
  (bind _skillanimation (`self.SkillAnimation`))
  (bind ((`CastimgTime_36_6EDFBF4641E634241F394591FF416122` _castimgtime)) (break `/Game/SkillSystem/Enum_Structure/s_SkillStage` (`self.GetCurrentStage`)))
  (bind ((`CastimgTime_36_6EDFBF4641E634241F394591FF416122` _castimgtime_2)) (break `/Game/SkillSystem/Enum_Structure/s_SkillStage` (`self.GetCurrentStage`)))
  (bind _returnvalue (`TimelineComponent.GetPlaybackPosition` (`self.Casting Timeline`)))
  (bind _mainwidget (`/Game/Blueprint/Character/Wizard/Wizard_Character.mainWidget` (`self.PlayerREF`)))
  (bind _mainwidget_2 (`/Game/Blueprint/Character/Wizard/Wizard_Character.mainWidget` (`self.PlayerREF`)))
  ;[1 1 1] 캐스팅바텍스트 및 애니메이션 재생
  (`/Engine/EditorBlueprintResources/StandardMacros.IsValid` _skillanimation
    (:`Is Valid`
      (`self.PlayAnimation` _skillanimation (/ (`AnimSequenceBase.SequenceLength` _skillanimation) _castimgtime)
        (:`Then`
          (`TextBlock.SetText` (`/Game/SkillSystem/Widget/W_Main.CastedSpeelText` _mainwidget) (`|FormatText` "Casting{SpellName}" (`.Name_9_C70043614A43644DEA2E35A66B08C621` (break `/Game/SkillSystem/Enum_Structure/s_SkillInfo` (`self.SKillInfo`)))))
          (`ProgressBar.SetPercent` (`/Game/SkillSystem/Widget/W_Main.CastingBar` _mainwidget) 0.0)
          (`TextBlock.SetText` (`/Game/SkillSystem/Widget/W_Main.CastTimeText` _mainwidget) (`|FormatText` "0.0 / {Cast Time}" (`KismetTextLibrary.Conv_DoubleToText` _castimgtime "HalfToEven" false true 1 324 1 1)))
          (`TimelineComponent.SetTimelineLength` (`self.Casting Timeline`) _castimgtime)
          (`Widget.SetVisibility` (`/Game/SkillSystem/Widget/W_Main.CastingBarMain` _mainwidget) "HitTestInvisible")
          (`Timeline|Casting Timeline` :!via `PlayFromStart`
            (:`Update`
              (`ProgressBar.SetPercent` (`/Game/SkillSystem/Widget/W_Main.CastingBar` _mainwidget_2) (/ _returnvalue _castimgtime_2))
              (`TextBlock.SetText` (`/Game/SkillSystem/Widget/W_Main.CastTimeText` _mainwidget_2) (`|FormatText` "{CurrentTime}/{CastTime}" (`KismetTextLibrary.Conv_DoubleToText` _returnvalue "HalfToEven" false true 1 324 1 1) (`KismetTextLibrary.Conv_DoubleToText` _castimgtime_2 "HalfToEven" false true 1 324 1 1))))
            (:`Finished`
              (`Widget.SetVisibility` (`/Game/SkillSystem/Widget/W_Main.CastingBarMain` _mainwidget_2) "Hidden"))))
        (:`Completed`
          (`self.OncastCompleted` :!label _label))))
    (:`Is Not Valid`
      (`KismetSystemLibrary.PrintString` (`KismetTextLibrary.Conv_TextToString` (`|FormatText` "Casting {Name}" (`.Name_9_C70043614A43644DEA2E35A66B08C621` (break `/Game/SkillSystem/Enum_Structure/s_SkillInfo` (`self.SKillInfo`))))) true true (struct :`G` 0.66 :`B` 1.0 :`A` 1.0) 0.5)
      (goto _label))))

(event `Initialize SpellCast`
  (bind _playerref (`self.PlayerREF`))
  (bind ((`ManaCost_44_4C078B0A4A4028F864CEA09F3DA6E744` _manacost)) (break `/Game/SkillSystem/Enum_Structure/s_SkillStage` (`self.GetCurrentStage`)))
  (if (>= (`.CurrentValue_7_2F63A7F6498A3A7B352ACBAAB7C9183F` (break `/Game/SkillSystem/Enum_Structure/s_StatData` (`/Game/Blueprint/Character/Wizard/Wizard_Character.GetStat` (`self.PlayerREF`) "NewEnumerator2"))) _manacost)
    (set `self.Currently Casted?` true)
    (`/Game/Blueprint/Character/Wizard/Wizard_Character.BeginSpellCast` _playerref self)
    (`/Game/Blueprint/Character/Wizard/Wizard_Character.ModifyStat` _playerref "NewEnumerator2" (* _manacost -1) true)
    (`self.OnSpellCast`)
    (else
      (`KismetSystemLibrary.PrintString` "nor enought mana" true true (struct :`R` 1.0 :`B` 0.092422 :`A` 1.0)))))

(event `OnTryCastSpell`
  (if (and (not (`self.OnCoolDown?`)) (not (`self.Currently Casted?`)) (not (`/Game/Blueprint/Character/Wizard/Wizard_Character.isCasting?` (`self.PlayerREF`))))
    (`self.Initialize SpellCast`)))

(event `OncastCompleted`
  (bind _hotkey (`self.HotKey`))
  (bind _cooldowntimeline (`self.CoolDownTimeline`))
  (bind _hotkey_2 (`self.HotKey`))
  (bind ((`CoolDown_35_BFB74E6540E57D658D294280315CF1F5` _cooldown)) (break `/Game/SkillSystem/Enum_Structure/s_SkillStage` (`self.GetCurrentStage`)))
  (bind _returnvalue (`TimelineComponent.GetPlaybackPosition` _cooldowntimeline))
  (bind _returnvalue_2 (`TimelineComponent.GetTimelineLength` _cooldowntimeline))
  (bind _cooldowntext (`/Game/SkillSystem/Widget/W_SkillHotkey.CoolDownText` _hotkey_2))
  (bind _returnvalue_3 (- _returnvalue_2 _returnvalue))
  (`/Game/Blueprint/Character/Wizard/Wizard_Character.EndSpellCast` (`self.PlayerREF`) self)
  (set `self.OnCoolDown?` true)
  (`KismetSystemLibrary.PrintString` "Spell On CoolDown" true true (struct :`R` 0.345456 :`G` 1.0 :`A` 1.0) 0.5)
  (set `self.Currently Casted?` false)
  (`/Engine/EditorBlueprintResources/StandardMacros.IsValid` _hotkey_2
    (:`Is Valid`
      (`Widget.SetIsEnabled` (`/Game/SkillSystem/Widget/W_SkillHotkey.SkillButton` _hotkey_2) false)
      (`Image.SetColorAndOpacity` (`/Game/SkillSystem/Widget/W_SkillHotkey.SkillIcon` _hotkey_2) (struct :`R` 0.33 :`G` 0.33 :`B` 0.33 :`A` 1.0))
      (`MaterialInstanceDynamic.SetScalarParameterValue` (`/Game/SkillSystem/Widget/W_SkillHotkey.SetCooldownMat` _hotkey_2) "Percent" 1.0)
      (`TextBlock.SetText` _cooldowntext (`KismetTextLibrary.Conv_DoubleToText` _cooldown "HalfToEven" false false 1 324 0 0))
      (`Widget.SetVisibility` _cooldowntext "HitTestInvisible")
      (`Widget.SetVisibility` (`/Game/SkillSystem/Widget/W_SkillHotkey.CooldownImage` _hotkey_2) "HitTestInvisible"))
    (:`Is Not Valid`
      _))
  (`TimelineComponent.SetTimelineLength` (`self.CoolDownTimeline`) _cooldown)
  (`Timeline|CoolDownTimeline` :!via `PlayFromStart`
    (:`Update`
      (`/Engine/EditorBlueprintResources/StandardMacros.IsValid` _hotkey
        (:`Is Valid`
          (`MaterialInstanceDynamic.SetScalarParameterValue` (`/Game/SkillSystem/Widget/W_SkillHotkey.SetCooldownMat` _hotkey) "Percent" (- 1.0 (/ _returnvalue _returnvalue_2)))
          (`TextBlock.SetText` (`/Game/SkillSystem/Widget/W_SkillHotkey.CoolDownText` _hotkey) (`KismetTextLibrary.Conv_DoubleToText` _returnvalue_3 "HalfToEven" false false 1 324 0 (select `bool` (> _returnvalue_3 1.0) :`false` 1))))))
    (:`Finished`
      (`self.OnCooldownExpired`))))

(event `OnCooldownExpired`
  (bind _hotkey (`self.HotKey`))
  (set `self.OnCoolDown?` false)
  (`/Engine/EditorBlueprintResources/StandardMacros.IsValid` _hotkey
    (:`Is Valid`
      (if (not (`/Game/SkillSystem/Widget/W_SkillHotkey.Deactivated?` _hotkey))
        (`Widget.SetIsEnabled` (`/Game/SkillSystem/Widget/W_SkillHotkey.SkillButton` _hotkey) true)
        (`Image.SetColorAndOpacity` (`/Game/SkillSystem/Widget/W_SkillHotkey.SkillIcon` _hotkey) (struct :`R` 1.0 :`G` 1.0 :`B` 1.0 :`A` 1.0)))
      (`Widget.SetVisibility` (`/Game/SkillSystem/Widget/W_SkillHotkey.CoolDownText` _hotkey) "Hidden")
      (`Widget.SetVisibility` (`/Game/SkillSystem/Widget/W_SkillHotkey.CooldownImage` _hotkey) "Hidden"))))

(event `OnSkillNotify`
  (`KismetSystemLibrary.PrintString` (`KismetTextLibrary.Conv_TextToString` (`|FormatText` "Casting {Name}" (`.Name_9_C70043614A43644DEA2E35A66B08C621` (break `/Game/SkillSystem/Enum_Structure/s_SkillInfo` (`self.SKillInfo`))))) true true (struct :`G` 0.66 :`B` 1.0 :`A` 1.0) 0.5)
  (`self.OncastCompleted`))

(fn `GetCurrentStage`
  (returns (Out :type "/Game/SkillSystem/Enum_Structure/s_SkillStage Structure"))
  (return (`|GetArrayItem` (`.Stages_23_2AFE02F542CFDAAEBF0E69AD5FF57DA0` (break `/Game/SkillSystem/Enum_Structure/s_SkillInfo` (`self.SKillInfo`))) (`self.CurrentStagelIndex`))))

(fn `UserConstructionScript`)