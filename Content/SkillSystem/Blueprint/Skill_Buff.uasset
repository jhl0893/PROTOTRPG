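; Base skill Blueprint for timed player buffs, with empty ApplyEffect and RemoveEffect events as hooks for the actual effect.
; On skill notify it resets an existing buff of the same class on the player, or applies the effect and registers a new one.
; A timeline sized to the current stage's duration drives the widget's countdown text and material percentage, then removes the effect and buff when finished.
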(event `self.OnSkillNotify`
  (bind (_out_ _found_buff) (`/Game/Blueprint/Character/Wizard/Wizard_Character.HasBuff?` (`self.PlayerREF`) (`GameplayStatics.GetObjectClass` self)))
  (`parent.OnSkillNotify`)
  (if _out_
    (`self.ResetBuff` _found_buff)
    (else
      (`self.OnActivated`))))

(event `ResetBuff`
  (bind _buffwidgetref (`self.buffwidgetREF`))
  (bind _output_get (set `self.Duration` (`.Duration_54_D24A97DF413FFE38015494AAEBAE643A` (break `/Game/SkillSystem/Enum_Structure/s_SkillStage` (`self.GetCurrentStage`))) :!label _label))
  (set `self.PassedTime` 0.0)
  (`TimelineComponent.SetTimelineLength` (`self.DurationTimeLine`) _output_get)
  (`Widget.SetVisibility` (`/Game/SkillSystem/Widget/W_Buff.DurationText` (`self.buffwidgetREF`)) "Visible")
  (`Widget.SetVisibility` (`/Game/SkillSystem/Widget/W_Buff.DurationMat` (`self.buffwidgetREF`)) "Visible")
  (`Timeline|DurationTimeLine` :`NewTime` 0.0 :!via `PlayFromStart`
    (:`Update`
      (set `self.PassedTime` (`TimelineComponent.GetPlaybackPosition` (`self.DurationTimeLine`)))
      (`TextBlock.SetText` (`/Game/SkillSystem/Widget/W_Buff.DurationText` _buffwidgetref) (`KismetTextLibrary.Conv_DoubleToText` (- (`self.Duration`) (`self.PassedTime`)) "HalfToZero" false false 1 324 0 0))
      (`MaterialInstanceDynamic.SetScalarParameterValue` (`/Game/SkillSystem/Widget/W_Buff.DynamicDurationMat` _buffwidgetref) "Percent" (/ (`self.PassedTime`) (`self.Duration`))))
    (:`Finished`
      (`self.OnDeactivated`))))

(event `OnActivated`
  (`self.ApplyEffect`)
  (bind _widget (`/Game/Blueprint/Character/Wizard/Wizard_Character.AddBuff` (`self.PlayerREF`) self))
  (set `self.buffwidgetREF` _widget)
  (goto _label))

(event `ApplyEffect`)

(event `RemoveEffect`)

(event `OnDeactivated`
  (`self.RemoveEffect`)
  (`/Game/Blueprint/Character/Wizard/Wizard_Character.RemoveBuff` (`self.PlayerREF`) self)
  (set `self.buffwidgetREF` null))

(fn `UserConstructionScript`
  (`parent.UserConstructionScript`))